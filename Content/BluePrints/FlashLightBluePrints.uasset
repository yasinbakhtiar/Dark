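; Flashlight Blueprint that switches its light component on at BeginPlay and then runs an endless, randomly timed flicker-style loop.
; After each random delay, nested coin flips pick between waiting, hiding the light then waiting, or calling TurnOnoffFlashlight with a random repeat range.
; Each branch feeds back into the delay, bypassing the initial switch-on, so a hidden light is not directly re-shown by this graph.
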(event EventBeginPlay
  (bind _returnvalue (Math|Random|RandomBool))
  (bind _returnvalue_2 (Math|Random|RandomFloatinRange 0.5 1.5))
  (bind _lightcomponent (Variables|Default|GetLightComponent))
  (Rendering|SetVisibility _lightcomponent true false)
  (Utilities|FlowControl|Delay (Math|Random|RandomFloatinRange 1.0 4.0) :!label _label)
  (if _returnvalue
    (if _returnvalue
      (Utilities|FlowControl|Delay _returnvalue_2)
      (goto _label)
      (else
        (Rendering|SetVisibility (Variables|Default|GetLightComponent) false false)
        (Utilities|FlowControl|Delay _returnvalue_2)
        (goto _label)))
    (else
      (Utilities|TurnOn-offFlashlight 1 (Math|Random|RandomIntegerinRange 2 5) _lightcomponent
        (:Complete
          (goto _label))))))

(fn ConstructionScript)